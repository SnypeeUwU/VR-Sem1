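; BP_Snowman is a snowman actor with a procedural running animation that toggles on and off with the space bar.
; While running, Tick advances a time value scaled by an animation speed and feeds it through a sine wave to pitch the hip and shoulder joints.
; Diagonal limb pairs swing in opposite phase.
; Toggling off freezes the limbs in their current pose.
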(event EventBeginPlay)

(event Collision|EventActorBeginOverlap
  (params (OtherActor :type Actor%20Object%20Reference)))

(event EventTick
  (params (DeltaSeconds :type Float%20%28single-precision%29))
  ;[0.15 0.15 0.15 0.5] For Animtaion
  (if (Variables|Default|GetIsRunning)
    (bind _output_get (Variables|Default|SetRunTime (+ (* DeltaSeconds (Variables|Default|GetAnimSpeed)) (Variables|Default|GetRunTime))))
    (Transformation|SetRelativeRotation (Variables|Default|GetLeftHipJoint) (Math|Rotator|MakeRotator 0.0 (* (Math|Trig|Sin(Radians) _output_get) (Variables|Default|GetSwingAngle)) 0.0) false false)
    (Transformation|SetRelativeRotation (Variables|Default|GetRightHipJoint) (Math|Rotator|MakeRotator 0.0 (* (* (Math|Trig|Sin(Radians) _output_get) (Variables|Default|GetSwingAngle)) -1.0) 0.0) false false)))

(event Input|KeyboardEvents|SpaceBar
  (params (Key :type Key%20Structure :default "None"))
  ;[0.15 0.15 0.15 0.5] For Input Trigger
  (:Pressed
    (Variables|Default|SetIsRunning (not (Variables|Default|GetIsRunning)))))

(fn ConstructionScript)